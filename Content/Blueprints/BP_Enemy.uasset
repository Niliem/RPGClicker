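; BP_Enemy is the battle enemy, one reusable actor that becomes each successive entry in its Wave list, repeating the last.
; It loads stats from DT_Enemies by row name and reports data and health to BP_BattleGameMode.
; Hit subtracts per-type Defence from a damage map, clamped at zero; death briefly hides the cube before the next entry loads.
; Tag-keyed action reactions are only printed.
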(event EventBeginPlay
  (CallFunction|Dead)
  (bind _asbp_battle_game_mode (Utilities|Casting|CastToBP_BattleGameMode (Game|GetGameMode)))
  (Variables|/Game/Blueprints/BP_BattleGameMode.BP_BattleGameMode_C|SetEnemy _asbp_battle_game_mode self)
  (CallFunction|InitEnemy (CallFunction|GetNextEnemy)))

(event EventHit
  (params (TakingDamage :type Map%20of%20EDamageType%20Enums%20to%20Float%20%28single-precision%29s :default "NewEnumerator0"))
  (if (Variables|Default|GetbCanTakeDamage)
    (Audio|PlaySound2D "/Engine/VREditor/Sounds/UI/Drop_Item_From_ContentBrowser.Drop_Item_From_ContentBrowser" 1.0 1.0 0.0 0 0)
    (CallFunction|PerformAction "(TagName=\"Action.TakeDamage\")")
    (bind _output_get (Variables|Default|SetCurrentHealth (- (Variables|Default|GetCurrentHealth) (CallFunction|CalculateTakingDamage TakingDamage))))
    (bind _asbp_battle_game_mode (Utilities|Casting|CastToBP_BattleGameMode (Game|GetGameMode)))
    (Default|UpdateEnemyHealth _asbp_battle_game_mode (Variables|Default|GetCurrentHealth))
    (if (<= _output_get 0.0)
      (CallFunction|Dead)
      (Utilities|FlowControl|Delay 0.2)
      (CallFunction|InitEnemy (CallFunction|GetNextEnemy)))))

(fn ConstructionScript)

(fn InitEnemy
  (params (RowName :type Name))
  (bind _returnvalue (Utilities|GetDataTableRow "/Game/Blueprints/DT_Enemies.DT_Enemies" RowName)
    (:then
      (bind _output_get (Variables|Default|SetCurrentEnemyData _returnvalue))
      (Variables|Default|SetCurrentHealth (.MaxHealth (Utilities|Struct|BreakS_EnemyData _output_get)))
      (Variables|Default|SetbCanTakeDamage true)
      (Rendering|SetVisibility (Variables|Default|GetCube) true false)
      (bind _asbp_battle_game_mode (Utilities|Casting|CastToBP_BattleGameMode (Game|GetGameMode)))
      (Default|SetEnemyData _asbp_battle_game_mode (Variables|Default|GetCurrentEnemyData)))))

(fn CalculateTakingDamage
  (params (TargetMap :type Map%20of%20EDamageType%20Enums%20to%20Float%20%28single-precision%29s :default "NewEnumerator0"))
  (bind _keys (Utilities|Map|Keys TargetMap))
  (for _array_element _keys
    (LocalVariables|Setl_FinalDamage (+ (LocalVariables|Getl_FinalDamage) (select (< (- (.Value (Utilities|Map|Find TargetMap _array_element)) (select (.ReturnValue (Utilities|Map|Find (.Defence (Utilities|Struct|BreakS_EnemyData (Variables|Default|GetCurrentEnemyData))) _array_element)) (.Value (Utilities|Map|Find (.Defence (Utilities|Struct|BreakS_EnemyData (Variables|Default|GetCurrentEnemyData))) _array_element)) 0.0)) 0.0) 0.0 (- (.Value (Utilities|Map|Find TargetMap _array_element)) (select (.ReturnValue (Utilities|Map|Find (.Defence (Utilities|Struct|BreakS_EnemyData (Variables|Default|GetCurrentEnemyData))) _array_element)) (.Value (Utilities|Map|Find (.Defence (Utilities|Struct|BreakS_EnemyData (Variables|Default|GetCurrentEnemyData))) _array_element)) 0.0))))))
  (return (LocalVariables|Getl_FinalDamage)))

(fn Dead
  (CallFunction|PerformAction "(TagName=\"Action.Death\")")
  (Variables|Default|SetbCanTakeDamage false)
  (Rendering|SetVisibility (Variables|Default|GetCube) false false))

(fn GetNextEnemy
  (Variables|Default|SetCurrentEnemy (select (== (Variables|Default|GetCurrentEnemy) (- (Utilities|Array|Length (Variables|Default|GetWave)) 1)) (- (Utilities|Array|Length (Variables|Default|GetWave)) 1) (+ (Variables|Default|GetCurrentEnemy) 1)))
  (return (Utilities|Array|Get(acopy) (Variables|Default|GetWave) (Variables|Default|GetCurrentEnemy))))

(fn PerformAction
  (params (ActionTag :type Gameplay%20Tag%20Structure))
  (bind _currentenemydata (Variables|Default|GetCurrentEnemyData))
  (bind _actions (Utilities|Struct|BreakS_EnemyData _currentenemydata))
  (bind (_value _returnvalue) (Utilities|Map|Find _actions ActionTag))
  (if _returnvalue
    (Development|PrintString (Utilities|String|ToString(Text) (Utilities|Struct|BreakS_Action _value)))))