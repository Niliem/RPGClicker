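; BP_BattleGameMode is a game mode for battles that links an enemy to the main battle UI.
; On BeginPlay it creates the UI_MainBattle widget for player 0, stores it and adds it to the viewport.
; Its Hit event forwards damage to the Enemy reference, while UpdateEnemyHealth and SetEnemyData pass enemy health and data through to the widget.
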(event EventHit
  (params (TakingDamage :type Map%20of%20EDamageType%20Enums%20to%20Float%20%28single-precision%29s :default "NewEnumerator0"))
  (Default|Hit (Variables|Default|GetEnemy) TakingDamage))

(event EventBeginPlay
  (bind _returnvalue (UserInterface|CreateWidget "/Game/Blueprints/UI_MainBattle.UI_MainBattle_C" (Game|GetPlayerController 0)))
  (bind _output_get (Variables|Default|SetUIMain _returnvalue))
  (UserInterface|Viewport|AddtoViewport _output_get 0))

(fn ConstructionScript)

(fn UpdateEnemyHealth
  (params (CurrentHealth :type Float%20%28single-precision%29))
  (Default|UpdateEnemyHealth (Variables|Default|GetUIMain) CurrentHealth))

(fn SetEnemyData
  (params (EnemyData :type S%20Enemy%20Data%20Structure))
  (Default|SetEnemyData (Variables|Default|GetUIMain) EnemyData))